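; Online player controller that handles chat, match UI and level changes for the modoGhosty game mode.
; It creates the chat widget at start, switches input mode for typing, relays messages to the game mode and adds authority-specific keyboard widgets when chat closes.
; An input triggers the game mode countdown; showcoutdown picks a random level to join through the game instance.
; Other events show name, victory/defeat and death screens, the latter possessing a camera actor.
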(event `self.ReceiveTick`
  (params (DeltaSeconds :type "Float (single-precision)")))

(event `cambiar nivel`
  (params (nivel :type String))
  (bind _asgame_instancia (cast `/Game/Blueprints/online/instance/game-instancia` (`GameplayStatics.GetGameInstance`)))
  (`/Game/Blueprints/online/instance/game-instancia.unir a nivel` _asgame_instancia nivel))

(event `self.ReceiveBeginPlay`
  (`|ExecutionSequence`
    (:`then_0`
      (`WidgetBlueprintLibrary.SetInputMode_GameOnly` self))
    (:`then_1`
      (`self.evento chat`))))

(event `InputAction|chat`
  (params (Key :type "Key Structure"))
  (:`Pressed`
    (`self.server chat` true :!label _label)))

(event `chat`
  (goto _label))

(event `showcoutdown`
  (bind _returnvalue (`|CreateWidget` "/Game/Blueprints/online/inicio/inicio-partida.inicio-partida_C"))
  (`UserWidget.AddToViewport` _returnvalue 0)
  (`KismetSystemLibrary.Delay` 5.0)
  (bind _asplayer_controller (cast `/Game/Blueprints/online/player-controller` (`GameplayStatics.GetPlayerController` 0)))
  (`self.cambiar nivel` _asplayer_controller (`KismetArrayLibrary.Array_Random` (`self.niveles`))))

(event `InputAction|cambio de nivel`
  (params (Key :type "Key Structure"))
  (:`Pressed`
    (bind _asmodo_ghosty (cast `/Game/personajes/gosthy/demond/Blueprint/modoGhosty` (`GameplayStatics.GetGameMode`) :!label _label_2))
    (`/Game/personajes/gosthy/demond/Blueprint/modoGhosty.coutdown` _asmodo_ghosty)))

(event `cambio-nivel`
  (goto _label_2))

(event `evento chat`
  ;[1 1 1] chat
  (bind _returnvalue (`|CreateWidget` "/Game/Blueprints/online/personajes/chat.chat_C" (`GameplayStatics.GetPlayerController` 0)))
  (bind _output_get (set `self.chatV` _returnvalue))
  (`UserWidget.AddToViewport` _output_get 0))

(event `server chat`
  (params (NewParam :type Boolean))
  ;[1 1 1] chat
  (`/Game/Blueprints/online/personajes/chat.setfocuschat` (`self.chatV`) NewParam)
  (if NewParam
    (`WidgetBlueprintLibrary.SetInputMode_GameAndUIEx` self (`self.chatV`))
    (else
      (`WidgetBlueprintLibrary.SetInputMode_GameOnly` self)
      (set `self.bShowMouseCursor` true)
      (`/Engine/EditorBlueprintResources/ActorMacros.Switch Has Authority`
        (:`Authority`
          (bind _returnvalue (`|CreateWidget` "/Game/Blueprints/interfaz-personajes/teclado-ghosty.teclado-ghosty_C" self))
          (`UserWidget.AddToViewport` _returnvalue 0))
        (:`Remote`
          (bind _returnvalue_2 (`|CreateWidget` "/Game/Blueprints/interfaz-personajes/teclado-ghosty1.teclado-ghosty1_C" self))
          (`UserWidget.AddToViewport` _returnvalue_2 0))))))

(event `server messaje`
  (params (NewParam :type String) (NewParam2 :type String))
  ;[1 1 1] chat
  (`|ExecutionSequence`
    (:`then_0`
      (bind _asmodo_ghosty (cast `/Game/personajes/gosthy/demond/Blueprint/modoGhosty` (`GameplayStatics.GetGameMode`)))
      (`/Game/personajes/gosthy/demond/Blueprint/modoGhosty.mensajes` _asmodo_ghosty NewParam NewParam2))))

(event `mensajesplayers`
  (params (NewParam :type String) (NewParam2 :type String))
  ;[1 1 1] chat
  (`/Game/Blueprints/online/personajes/chat.menssajeswid` (`self.chatV`) NewParam NewParam2))

(event `derr`
  (set `self.victoria` false)
  ;[1 1 1] chat
  (`WidgetLayoutLibrary.RemoveAllWidgets`)
  (bind _returnvalue (`|CreateWidget` "/Game/Blueprints/VICTORIA.VICTORIA_C"))
  (`UserWidget.AddToViewport` _returnvalue 0)
  (`KismetSystemLibrary.Delay` 14.0)
  (bind _asgame_instancia (cast `/Game/Blueprints/online/instance/game-instancia` (`GameplayStatics.GetGameInstance`)))
  (`/Game/Blueprints/online/instance/game-instancia.unir a nivel` _asgame_instancia "nivel_1"))

(event `vict-derr`
  (params (victoria :type Boolean))
  (set `self.victoria` false)
  (`WidgetLayoutLibrary.RemoveAllWidgets`)
  (bind _returnvalue (`|CreateWidget` "/Game/Blueprints/VICTORIA.VICTORIA_C" null victoria))
  (`UserWidget.AddToViewport` _returnvalue 0))

(event `nombre`
  (bind _returnvalue (`|CreateWidget` "/Game/Blueprints/online/personajes/nombre.nombre_C"))
  (`UserWidget.AddToViewport` _returnvalue 0))

(event `evmuerte`
  (if (`self.victoria`)
    (`WidgetLayoutLibrary.RemoveAllWidgets`)
    (bind _returnvalue (`|CreateWidget` "/Game/Blueprints/muerte.muerte_C"))
    (`UserWidget.AddToViewport` _returnvalue 0)
    (bind _returnvalue_2 (`GameplayStatics.GetActorOfClass` "/Game/actores/extras/camara.camara_C"))
    (`self.Possess` (`GameplayStatics.GetPlayerController` 0) _returnvalue_2)))

(event `visibilidad`
  (params (Meta2 :type "Widget Object Reference"))
  (`/Engine/EditorBlueprintResources/ActorMacros.Switch Has Authority`
    (:`Authority`
      (`Widget.SetVisibility` Meta2 "Visible")
      (`KismetSystemLibrary.Delay` 4.0)
      (`Widget.SetVisibility` Meta2 "Hidden"))
    (:`Remote`
      (`Widget.SetVisibility` Meta2 "Hidden"))))

(fn `savegamesheck`)

(fn `UserConstructionScript`)